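; BP_rect moves StaticMesh2 around a square loop in the relative XZ plane while playback is enabled.
; Tick switches on the Movetype enum (Right, Up, Left, Down), stepping LocX or LocZ by a fixed, frame-rate-dependent amount and setting relative location.
; Each case advances Movetype to the next side when its coordinate reaches or passes a hardcoded limit.
; DOPLAY sets the ISPLAY flag that gates the motion.
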(event EventTick
  (params (DeltaSeconds :type Float%20%28single-precision%29))
  (if (Variables|Default|GetISPLAY)
    ;[1 1 1] 두가지 이상의 선택지가 필요할땐
    ; ENUM (열거형을 만들고 )  스위치를 생성한다
    (switch Utilities|FlowControl|Switch|SwitchonEN_movetype (Variables|Default|Getmovetype)
      (:NewEnumerator0
        (bind _output_get (Variables|Default|Setloc%20x (+ (Variables|Default|Getloc%20x) 1.0)))
        (Transformation|SetRelativeLocation (Variables|Default|GetStaticMesh2) (Math|Vector|MakeVector _output_get 0.0 0.0) false false)
        (if (>= (Variables|Default|Getloc%20x) 2e+02)
          (Variables|Default|Setmovetype "NewEnumerator1")))
      (:NewEnumerator1
        (bind _output_get_2 (Variables|Default|Setloc%20z (+ (Variables|Default|Getloc%20z) 1.0)))
        (Transformation|SetRelativeLocation (Variables|Default|GetStaticMesh2) (Math|Vector|MakeVector (Variables|Default|Getloc%20x) 0.0 _output_get_2) false false)
        (if (>= (Variables|Default|Getloc%20z) 2e+02)
          (Variables|Default|Setmovetype "NewEnumerator2")))
      (:NewEnumerator2
        (bind _output_get_3 (Variables|Default|Setloc%20x (- (Variables|Default|Getloc%20x) 1.0)))
        (Transformation|SetRelativeLocation (Variables|Default|GetStaticMesh2) (Math|Vector|MakeVector _output_get_3 0.0 (Variables|Default|Getloc%20z)) false false)
        (if (<= (Variables|Default|Getloc%20x) 0.0)
          (Variables|Default|Setmovetype "NewEnumerator3")))
      (:NewEnumerator3
        (bind _output_get_4 (Variables|Default|Setloc%20z (- (Variables|Default|Getloc%20z) 1.0)))
        (Transformation|SetRelativeLocation (Variables|Default|GetStaticMesh2) (Math|Vector|MakeVector (Variables|Default|Getloc%20x) 0.0 _output_get_4) false false)
        (if (< (Variables|Default|Getloc%20z) 0.0)
          (Variables|Default|Setmovetype "NewEnumerator0"))))))

(fn ConstructionScript)

(fn DOPLAY
  (params (IsPlay :type Boolean))
  (Variables|Default|SetISPLAY IsPlay)
  (return false))